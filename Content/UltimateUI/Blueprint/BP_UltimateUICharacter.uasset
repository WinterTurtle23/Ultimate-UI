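; BP_UltimateUICharacter is a player character for the UltimateUI project that sets up and responds to Enhanced Input.
; On BeginPlay it casts its controller to PC_UltimateUI and adds the IMC_UltimateUI mapping context.
; The Jump action triggers a jump, while Move, Ability and Crouch only print debug strings as placeholders.
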(event Input|EnhancedActionEvents|EnhancedInputActionIA_Move
  (params (ActionValue :type Boolean) (ElapsedSeconds :type Float%20%28double-precision%29) (TriggeredSeconds :type Float%20%28double-precision%29) (InputAction :type Input%20Action%20Object%20Reference :default "/Game/UltimateUI/Inputs/Input/IA_Move.IA_Move"))
  (:Started
    (Development|PrintString "move")))

(event Input|EnhancedActionEvents|EnhancedInputActionIA_Ability
  (params (ActionValue :type Boolean) (ElapsedSeconds :type Float%20%28double-precision%29) (TriggeredSeconds :type Float%20%28double-precision%29) (InputAction :type Input%20Action%20Object%20Reference :default "/Game/UltimateUI/Inputs/Input/IA_Ability.IA_Ability"))
  (:Started
    (Development|PrintString "Ability")))

(event Input|EnhancedActionEvents|EnhancedInputActionIA_Crouch
  (params (ActionValue :type Boolean) (ElapsedSeconds :type Float%20%28double-precision%29) (TriggeredSeconds :type Float%20%28double-precision%29) (InputAction :type Input%20Action%20Object%20Reference :default "/Game/UltimateUI/Inputs/Input/IA_Crouch.IA_Crouch"))
  (:Started
    (Development|PrintString "Crouch")))

(event Input|EnhancedActionEvents|EnhancedInputActionIA_Jump
  (params (ActionValue :type Boolean) (ElapsedSeconds :type Float%20%28double-precision%29) (TriggeredSeconds :type Float%20%28double-precision%29) (InputAction :type Input%20Action%20Object%20Reference :default "/Game/UltimateUI/Inputs/Input/IA_Jump.IA_Jump"))
  (:Started
    (Character|Jump)))

(event EventBeginPlay
  (bind _aspc_ultimate_ui (Utilities|Casting|CastToPC_UltimateUI (Pawn|GetController)))
  (Utilities|IsValid (PlayerController|LocalPlayerSubsystems|GetEnhancedInputLocalPlayerSubsystem _aspc_ultimate_ui)
    (:Is%20Valid
      (Input|AddMappingContext (PlayerController|LocalPlayerSubsystems|GetEnhancedInputLocalPlayerSubsystem _aspc_ultimate_ui) "/Game/UltimateUI/Inputs/IMC_UltimateUI.IMC_UltimateUI" 0 "(bIgnoreAllPressedKeysUntilRelease=True,bForceImmediately=False,bNotifyUserSettings=False)"))))

(fn ConstructionScript)